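; BP_Enemy is an enemy that takes damage and shows its health through a widget.
; An ActorStats component holds health, and any damage received is passed to it to decrease that value.
; On BeginPlay and after each hit, UpdateHealthWidget casts the HealthWidget's content to WB_EnemyHealth and pushes the current health percentage.
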(event Game|Damage|EventAnyDamage
  (params (Damage :type Float%20%28single-precision%29) (DamageType :type Damage%20Type%20Object%20Reference) (InstigatedBy :type Controller%20Object%20Reference) (DamageCauser :type Actor%20Object%20Reference))
  (Class|ActorStats|DecreaseHeath (Variables|Default|GetActorStats) Damage)
  (CallFunction|UpdateHealthWidget))

(event EventBeginPlay
  (CallFunction|UpdateHealthWidget))

(fn ConstructionScript)

(fn UpdateHealthWidget
  (bind _aswb_enemy_health (Utilities|Casting|CastToWB_EnemyHealth (UserInterface|GetWidget (Variables|Default|GetHealth%20Widget))))
  (Default|UpdateHealthValue _aswb_enemy_health (Class|ActorStats|GetPercentageHealt (Variables|Default|GetActorStats))))