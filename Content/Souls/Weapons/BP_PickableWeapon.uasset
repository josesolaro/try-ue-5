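; BP_PickableWeapon is a weapon pickup that the third-person character collects on touch.
; The construction script sets the static mesh from WeaponData, so the pickup's look follows its data.
; When a BP_ThirdPersonCharacter overlaps the capsule, it calls that character's PickWeapon with the pickup actor itself, plus the parent socket and damage from WeaponData.
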(event OnComponentBeginOverlap(Capsule)
  (params (OverlappedComponent :type Primitive%20Component%20Object%20Reference) (OtherActor :type Actor%20Object%20Reference) (OtherComp :type Primitive%20Component%20Object%20Reference) (OtherBodyIndex :type Integer) (bFromSweep :type Boolean) (SweepResult :type Hit%20Result%20Structure%20%28by%20ref%29))
  (bind _asbp_third_person_character (Utilities|Casting|CastToBP_ThirdPersonCharacter OtherActor))
  (Class|SoulslikeCharacter|PickWeapon _asbp_third_person_character (Components|GetOwner OverlappedComponent) (Utilities|String|StringToName (Variables|/Game/Souls/Weapons/DA_Weapon.DA_Weapon_C|GetParentSocket (Variables|Default|GetWeapon%20Data))) (Variables|/Game/Souls/Weapons/DA_Weapon.DA_Weapon_C|GetDamage (Variables|Default|GetWeapon%20Data))))

(fn ConstructionScript
  (Components|StaticMesh|SetStaticMesh (Variables|Default|GetStaticMesh) (Variables|/Game/Souls/Weapons/DA_Weapon.DA_Weapon_C|GetStaticAsset (Variables|Default|GetWeapon%20Data))))